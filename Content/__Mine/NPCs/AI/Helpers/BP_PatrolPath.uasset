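; BP_PatrolPath is a spline-based patrol route actor for NPC AI, tracking the current point and travel direction.
; GetCurrentPoint returns that spline point's world location.
; IncrementPoint steps the index along the current direction, wrapping to the start past the end of a closed loop, or clamping and reversing at the ends of an open path.
; The event graph and construction script are empty.
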(event EventBeginPlay)

(event Collision|EventActorBeginOverlap
  (params (OtherActor :type Actor%20Object%20Reference)))

(event EventTick
  (params (DeltaSeconds :type Float%20%28single-precision%29)))

(fn ConstructionScript)

(fn GetCurrentPoint
  (return (Spline|GetLocationatSplinePoint (Variables|Default|GetPath) (Variables|Default|GetCurrentPoint) "World")))

(fn IncrementPoint
  (bind _path (Variables|Default|GetPath))
  (bind _returnvalue (Spline|GetNumberOfSplinePoints _path))
  (switch Utilities|FlowControl|Switch|SwitchonENUM_PatrolIncrementDirection (Variables|Default|GetDirection)
    (:NewEnumerator0
      (bind _result (Math|Integer|IncrementInt (Variables|Default|GetCurrentPoint))
        (:%20%20
          (if (> _result (- _returnvalue 1))
            (if (Class|SplineComponent|IsClosedLoop _path)
              (Variables|Default|SetCurrentPoint 0)
              (else
                (Variables|Default|SetCurrentPoint (- _returnvalue 1))
                (Variables|Default|SetDirection "NewEnumerator1")))))))
    (:NewEnumerator1
      (bind _result_2 (Math|Integer|DecrementInt (Variables|Default|GetCurrentPoint))
        (:%20%20
          (if (< _result_2 0)
            (Variables|Default|SetCurrentPoint 0)
            (Variables|Default|SetDirection "NewEnumerator0")))))))