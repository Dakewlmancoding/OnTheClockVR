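; Base NPC character that takes impact damage, such as punches and thrown objects, and ragdolls at zero health.
; Capsule hits from actors not tagged NPCNoHit apply self-damage from impulse magnitude, with a steeper multiplier for strong impacts.
; Ragdoll enables mesh physics, changes the NPC AI controller's state, then disables capsule collision.
; The construction script sets the Metahuman child actor class and owns that actor.
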(event OnComponentHit(CapsuleComponent)
  (params (HitComponent :type Primitive%20Component%20Object%20Reference) (OtherActor :type Actor%20Object%20Reference) (OtherComp :type Primitive%20Component%20Object%20Reference) (NormalImpulse :type Vector :default "0, 0, 0") (Hit :type Hit%20Result%20Structure%20%28by%20ref%29))
  (bind _returnvalue (Math|Vector|VectorLength NormalImpulse))
  (bind _returnvalue_2 (< _returnvalue 1e+03))
  (bind _returnvalue_3 (/ _returnvalue 1e+02))
  (bind _returnvalue_4 (/ _returnvalue 1e+01))
  (bind _returnvalue_5 (Math|Float|SelectFloat _returnvalue_3 _returnvalue_4 _returnvalue_2))
  ;[0.15 0.15 0.15 0.5] Punch and Thrown object damage
  (if (not (Actor|ActorHasTag OtherActor "NPCNoHit"))
    (Game|Damage|ApplyDamage self _returnvalue_5 0 0)
    (Development|PrintString (Utilities|String|Append (Utilities|GetDisplayName OtherActor) " dealt " (Utilities|String|ToString(Float) _returnvalue_5)))))

(event Custom|Ragdoll
  (Physics|SetSimulatePhysics (Variables|Character|GetMesh) true)
  (bind _asaicon_npc (Utilities|Casting|CastToAICON_NPC (AI|GetAIController self)))
  (Default|ChangeState _asaicon_npc (Utilities|Enum|LiteralenumENUM_NPCState "NewEnumerator6"))
  (Collision|SetCollisionEnabled (Variables|Collision|GetCapsuleComponent) "NoCollision"))

(event Game|Damage|EventAnyDamage
  (params (Damage :type Float%20%28single-precision%29) (DamageType :type Damage%20Type%20Object%20Reference) (InstigatedBy :type Controller%20Object%20Reference) (DamageCauser :type Actor%20Object%20Reference))
  (bind _output_get (Variables|Default|SetHealth (- (Variables|Default|GetHealth) Damage)))
  (Development|PrintString (Utilities|String|Append "HP at " (Utilities|String|ToString(Float) _output_get)))
  (if (<= _output_get 0.0)
    (CallFunction|Ragdoll)))

(fn ConstructionScript
  (ChildActorComponent|SetChildActorClass (Variables|Default|GetMetahuman) (Variables|Default|GetBaseMetahuman))
  (Actor|SetOwner (Variables|/Script/Engine.ChildActorComponent|GetChildActor (Variables|Default|GetMetahuman)) self))