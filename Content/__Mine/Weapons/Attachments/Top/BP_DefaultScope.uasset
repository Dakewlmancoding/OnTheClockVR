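; BP_DefaultScope is a top weapon attachment that provides a picture-in-picture scope view.
; Its construction script creates a render target for a SceneCaptureComponent2D and feeds it into a dynamic M_ScopeView material instance on the Plane mesh.
; When its parent actor is a BP_GunBase, it moves the capture component to the gun's Muzzle location, so the view originates there.
; All logic runs at construction; the event graph is empty.
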(event EventBeginPlay)

(event Collision|EventActorBeginOverlap
  (params (OtherActor :type Actor%20Object%20Reference)))

(event EventTick
  (params (DeltaSeconds :type Float%20%28single-precision%29)))

(fn ConstructionScript
  (|CallParentFunction)
  (bind _returnvalue (Rendering|CreateRenderTarget2D 1024 1024 "RTF_RGBA16f"))
  (bind _output_get (Variables|/Script/Engine.SceneCaptureComponent2D|SetTextureTarget (Variables|Default|GetSceneCaptureComponent2D) _returnvalue))
  (bind _returnvalue_2 (Rendering|Material|CreateDynamicMaterialInstance (Variables|Default|GetPlane) 0 "/Game/__Mine/Weapons/Attachments/Top/M_ScopeView.M_ScopeView" "ScopeView" :!class /Script/Engine.PrimitiveComponent))
  (Rendering|Material|SetTextureParameterValue _returnvalue_2 "RenderTargetParam" _output_get)
  (bind _asbp_gun_base (Utilities|Casting|CastToBP_GunBase (Actor|GetParentActor)))
  (Transformation|SetWorldLocation (Variables|Default|GetSceneCaptureComponent2D) (Transformation|GetWorldLocation (Variables|/Game/__Mine/Weapons/BP_GunBase.BP_GunBase_C|GetMuzzle _asbp_gun_base)) false false))