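; BP_VRHandCollider is a physics-driven collider that follows a VR hand motion controller.
; AttachCollider grabs the HandCollider component with a PhysicsHandle at a location and rotation offset and stores the given motion controller.
; Every Tick moves the handle's target to that controller's world location and rotation, so the collider trails the hand through physics rather than being rigidly attached.
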(event EventTick
  (params (DeltaSeconds :type Float%20%28single-precision%29))
  (bind _motioncontroller (Variables|Default|GetMotionController))
  (bind _returnvalue (Transformation|GetWorldTransform _motioncontroller))
  (Class|PhysicsHandleComponent|SetTargetLocationandRotation (Variables|Default|GetPhysicsHandle) (.location _returnvalue) (.rotation _returnvalue)))

(fn ConstructionScript)

(fn AttachCollider
  (params (HandMotionController :type Motion%20Controller%20Component%20Object%20Reference) (RotationOffcet :type Rotator) (LocationOffset :type Vector))
  (bind _handcollider (Variables|Default|GetHandCollider))
  (Physics|Components|PhysicsHandle|GrabComponentatLocationwithRotation (Variables|Default|GetPhysicsHandle) _handcollider "None" (+ LocationOffset (.location (Transformation|GetWorldTransform _handcollider))) RotationOffcet)
  (Variables|Default|SetMotionController HandMotionController))